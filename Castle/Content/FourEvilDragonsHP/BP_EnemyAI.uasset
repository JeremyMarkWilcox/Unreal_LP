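; Enemy AI for a dragon-game foe that chases the player and takes hits, driven by pawn sensing.
; Sighting a pawn triggers FollowPawn, which moves toward the player and calls an empty MeleeAttack on arrival.
; HitReact subtracts fixed damage, then resumes the chase or sets Dead.
; Death runs only when FollowPawn next sees Dead, destroying the actor immediately after starting its animation; the attack-animation chain is unconnected.
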(event OnSeePawn(PawnSensing)
  (params (Pawn :type Pawn%20Object%20Reference))
  (CallFunction|FollowPawn))

(event Custom|MeleeAttack
  ;[1 0.01562 0.01562 0.199] Enemy Attack
)

(event Custom|Death
  ;[0.2135 0.001112 0.001112 0.335] Death
  (Components|Animation|PlayAnimation (Variables|Character|GetMesh) "/Game/FourEvilDragonsHP/Animations/DragonTheNightmare/DieAnim.DieAnim" false)
  (Components|Timeline|SetPlayRate (Variables|Character|GetMesh) 1e+02)
  (Actor|DestroyActor))

(event Custom|FollowPawn
  ;[1 1 1 0.492] Movement
  (Components|Animation|PlayAnimation (Variables|Character|GetMesh) "/Game/FourEvilDragonsHP/Animations/DragonTheNightmare/WalkAnim.WalkAnim" false)
  (if (Variables|Default|GetDead)
    (CallFunction|Death)
    (else
      (AI|AIMoveTo self "0, 0, 0" (Game|GetPlayerCharacter 0) 2e+02 true
        (:OnSuccess
          (CallFunction|MeleeAttack))))))

(event Custom|HitReact
  ;[1 0.5602 0.0349] HitReact
  (if (not (Variables|Default|GetDead))
    (if (not (Variables|Default|GetGettingHit))
      (Variables|Default|SetGettingHit true)
      (Components|Animation|PlayAnimation (Variables|Character|GetMesh) "/Game/FourEvilDragonsHP/Animations/DragonTheNightmare/GetHitAnim.GetHitAnim" false)
      (bind _output_get (Variables|Default|SetHealth (- (Variables|Default|GetHealth) 1e+02)))
      (Development|PrintString (Utilities|String|ToString(Float) _output_get))
      (if (<= (Variables|Default|GetHealth) 0.0)
        (Variables|Default|SetDead true)
        (else
          (Variables|Default|SetGettingHit false)
          (CallFunction|FollowPawn))))))

(fn ConstructionScript)